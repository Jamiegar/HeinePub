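; COM_Sound is a sound component with one function per game audio event: workstation placement, pouring, serving, bell, music and bar fights.
; Most play non-positional 2D sounds, with placement picking randomly from an array.
; Pour-quality switches currently play the same sound for every result.
; Music functions spawn sounds with no asset set, bar fight start is an empty stub, and bar fight end stops its audio after a delay.
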(fn `SF_Bar Fight End`
  (if true
    (`AudioComponent.StopDelayed` (`self.Bar fight Var`) 1.0)))

(fn `SF_Bar Fight Start`
  (params (`Init?` :type Boolean))
  (if `Init?`
    _))

(fn `SF_Bell`
  (`GameplayStatics.SpawnSound2D` "/Game/Blueprint/Sounds/SoundFiles/CUE/Bell_Sound_Cue.Bell_Sound_Cue" 1.0 1.0 0.0 null))

(fn `SF_GameplayMusic`
  (`GameplayStatics.SpawnSound2D` null 1.0 1.0 0.0 null))

(fn `SF_MenuMusic`
  (`GameplayStatics.SpawnSound2D` null 1.0 1.0 0.0 null))

(fn `SF_PourPintEnd`
  (params (`Pour Type` :type "/Game/Blueprint/WorkStations/PourTypes/E_PourType Enum" :default "NewEnumerator0"))
  (switch `/Game/Blueprint/WorkStations/PourTypes/E_PourType` `Pour Type`
    (:`NewEnumerator0`
      (`GameplayStatics.PlaySound2D` "/Game/Blueprint/Sounds/SoundFiles/CUE/DrinkFillDone.DrinkFillDone" 1.0 1.0 0.0 null null))
    (:`NewEnumerator1`
      (`GameplayStatics.PlaySound2D` "/Game/Blueprint/Sounds/SoundFiles/CUE/DrinkFillDone.DrinkFillDone" 1.0 1.0 0.0 null null))
    (:`NewEnumerator2`
      (`GameplayStatics.PlaySound2D` "/Game/Blueprint/Sounds/SoundFiles/CUE/DrinkFillDone.DrinkFillDone" 1.0 1.0 0.0 null null))))

(fn `SF_ServingOrder`
  (params (`Pour Type` :type "/Game/Blueprint/WorkStations/PourTypes/E_PourType Enum" :default "NewEnumerator0"))
  (bind _servingordersound (`self.ServingOrderSound`))
  (switch `/Game/Blueprint/WorkStations/PourTypes/E_PourType` `Pour Type`
    (:`NewEnumerator0`
      (`GameplayStatics.PlaySound2D` _servingordersound 1.0 1.0 0.0 null null))
    (:`NewEnumerator1`
      (`GameplayStatics.PlaySound2D` _servingordersound 1.0 1.0 0.0 null null))
    (:`NewEnumerator2`
      (`GameplayStatics.PlaySound2D` _servingordersound 1.0 1.0 0.0 null null)))
  (`KismetSystemLibrary.PrintString` "Order Served Sound"))

(fn `SF_WorkstationPlacement`
  (`GameplayStatics.PlaySound2D` (`KismetArrayLibrary.Array_Random` (`self.WorkstaionPlacementSounds`)) 1.0 1.0 0.0 null null)
  (`KismetSystemLibrary.PrintString` "Playing Sound"))