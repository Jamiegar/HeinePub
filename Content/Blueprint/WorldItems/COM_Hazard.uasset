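; COM_Hazard applies environmental hazard effects to an actor, with water as the one handled type.
; ActivateHazard validates and stores the actor, then routes to WaterHazard, which starts a looping timer on activation.
; WaterSlow steps the bartender character's max walk speed down, clearing the timer once it reaches a floor.
; Deactivation restores a fixed walk speed but does not clear the timer.
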(event `Activate Hazard`
  (params (Hazard :type Name) (Activate :type Boolean) (Actor :type "Actor Object Reference"))
  ;[1 0.5449 0] Init the certain Hazard
  (`/Engine/EditorBlueprintResources/StandardMacros.IsValid` Actor
    (:`Is Valid`
      (bind _output_get (set `self.ActorRef` Actor))
      (switch `name` Hazard
        (:`Water`
          (`self.WaterHazard` Activate _output_get))))
    (:`Is Not Valid`
      (`KismetSystemLibrary.PrintString` "Actor Not Valid"))))

(event `WaterSlow`
  ;[1 0.2806 0] Water Slow Event (Cause cant use timeline :( )
  (bind _bartendercharacter (message `/Game/Blueprint/Interfaces/BPI_PlayerCharacter.GetBartenderCharacter` (`self.ActorRef`)))
  (bind _charactermovement (`Character.CharacterMovement` _bartendercharacter))
  (bind _result (`/Engine/EditorBlueprintResources/StandardMacros.DecrementFloat` (- (`CharacterMovementComponent.MaxWalkSpeed` _charactermovement) 100.0))
    (:`  `
      (bind _output_get (set `CharacterMovementComponent.MaxWalkSpeed` _result _charactermovement))
      (if (<= _output_get 200.0)
        (`KismetSystemLibrary.K2_ClearAndInvalidateTimerHandle` (`self.WaterSlowTimerRef`))))))

(fn `WaterHazard`
  (params (`Active?` :type Boolean) (Actor :type "Actor Object Reference"))
  (if `Active?`
    (bind _returnvalue (`KismetSystemLibrary.K2_SetTimerDelegate` (`|CreateDelegate` :!event `WaterSlow`) 0.2 true))
    (set `self.WaterSlowTimerRef` _returnvalue)
    (else
      (bind _bartendercharacter (message `/Game/Blueprint/Interfaces/BPI_PlayerCharacter.GetBartenderCharacter` Actor))
      (set `CharacterMovementComponent.MaxWalkSpeed` 600.0 (`Character.CharacterMovement` _bartendercharacter)))))