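; World item Blueprint that builds a wire-like mesh along its WireSpline component.
; The construction script adds one spline mesh component for each segment between neighboring spline points.
; Each component takes its start and end from the local-space locations and tangents of those points, so it follows the curve, and attaches to the default scene root.
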(fn `UserConstructionScript`
  (bind _wirespline (`self.WireSpline`))
  (for _index (range (+ (- (`SplineComponent.GetNumberOfSplinePoints` (`self.WireSpline`)) 2) 1))
    (bind _returnvalue (`AddComponent|NODE_AddSplineMeshComponent-0`))
    (bind (_location _tangent) (`SplineComponent.GetLocationAndTangentAtSplinePoint` _wirespline _index "Local"))
    (bind (_location_2 _tangent_2) (`SplineComponent.GetLocationAndTangentAtSplinePoint` _wirespline (+ _index 1) "Local"))
    (`SplineMeshComponent.SetStartAndEnd` _returnvalue _location _tangent _location_2 _tangent_2 true)
    (`SceneComponent.K2_AttachToComponent` _returnvalue (`self.DefaultSceneRoot`) "None" "KeepRelative" "KeepRelative" "KeepRelative" true)))