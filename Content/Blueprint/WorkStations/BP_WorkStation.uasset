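; BP_WorkStation is a data-driven workstation actor that players interact with, configured by a WorkstationData asset.
; The construction script applies the asset's mesh, or prints a red error when the asset is invalid.
; BeginPlay and Init both add the interaction logic component class named in the asset and store the instance.
; OnInteraction forwards the interacting actor to that component, keeping per-station behavior out of the actor.
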(event `self.ReceiveBeginPlay`
  (bind _returnvalue (`|AddComponentByClass` (`/Game/Blueprint/WorkStations/DataAsset/DA_WorkstationData.InteractionLogicComponent` (`self.WorkstationData`)) :!label _label))
  (set `self.WorkstationInteration` _returnvalue))

(event `/Game/Blueprint/Interfaces/BPI_Initalizable.Init`
  (goto _label))

(event `/Game/Blueprint/Interfaces/BPI_Interactable.OnInteraction`
  (params (InteractedActor :type "Actor Object Reference"))
  (`/Game/Blueprint/WorkStations/InteractableComponets/COM_WorkstationInteraction.PlayerInteract` (`self.WorkstationInteration`) InteractedActor))

(fn `UserConstructionScript`
  (`/Engine/EditorBlueprintResources/StandardMacros.IsValid` (`self.WorkstationData`)
    (:`Is Valid`
      (`StaticMeshComponent.SetStaticMesh` (`self.StaticMesh`) (`/Game/Blueprint/WorkStations/DataAsset/DA_WorkstationData.Mesh` (`self.WorkstationData`))))
    (:`Is Not Valid`
      (`KismetSystemLibrary.PrintString` "ERROR: Data Asset Empty" true true (struct :`R` 1.0 :`A` 1.0)))))