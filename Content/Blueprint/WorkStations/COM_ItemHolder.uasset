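; COM_ItemHolder is a workstation component that lets its owner hold and display a single item.
; Adding valid item data spawns a BP_Item at a named socket transform obtained through messages to the owner, attaches it to the owner, initializes it and stores the data.
; Removal destroys that actor and clears the held data, which query functions expose.
; Adding does not check for an already held item.
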(fn `AddItemToHolder`
  (params (Item :type "/Game/Blueprint/Items/ItemData/DA_ItemData Object Reference"))
  (`/Engine/EditorBlueprintResources/StandardMacros.IsValid` Item
    (:`Is Valid`
      (bind _socketexists (message `/Game/Blueprint/Interfaces/BPI_ItemContainer.DoesSocketExist` (`self.GetOwner`) (`self.Item Attachment Name`)))
      (if _socketexists
        (bind _sockettransform (message `/Game/Blueprint/Interfaces/BPI_ItemContainer.GetTransformOfSocket` (`self.GetOwner`) (`self.Item Attachment Name`)))
        (bind _returnvalue (`|SpawnActorFromClass` "/Game/Blueprint/Items/BP_Item.BP_Item_C" _sockettransform "Undefined" "OverrideRootScale" null (`local.Item`) null))
        (bind _output_get (set `self.ItemActor` _returnvalue))
        (`Actor.K2_AttachToActor` _output_get (`self.GetOwner`) "None" "KeepWorld" "KeepWorld" "KeepWorld" true)
        (message `/Game/Blueprint/Interfaces/BPI_Initalizable.Init` (`self.ItemActor`))
        (set `self.HeldItem` (`local.Item`))))))

(fn `GetHeldItem`
  (returns (HeldItem :type "/Game/Blueprint/Items/ItemData/DA_ItemData Object Reference"))
  (return (`self.HeldItem`)))

(fn `IsHoldingItem`
  (returns (IsHoldingItem :type Boolean))
  (return (`KismetSystemLibrary.IsValid` (`self.HeldItem`))))

(fn `RemoveItemFromHolder`
  (if (`self.IsHoldingItem`)
    (`Actor.K2_DestroyActor` (`self.ItemActor`))
    (set `self.HeldItem` null)))