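; BP_Waterfloor is a wet floor workstation hazard that changes the bartender character's walk speed while it overlaps the Box.
; Begin overlap stores the character through a GetBartenderCharacterMessage call and plays the WaterSlowDown timeline, which drives MaxWalkSpeed.
; End overlap resets that speed instantly to a hardcoded value, leaving the timeline-based SpeedUp event uncalled within this Blueprint.
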(event `self.Box.OnComponentBeginOverlap`
  (params (OverlappedComponent :type "PrimitiveComponent Object Reference") (OtherActor :type "Actor Object Reference") (OtherComp :type "PrimitiveComponent Object Reference") (OtherBodyIndex :type Integer) (bFromSweep :type Boolean) (SweepResult :type "HitResult Structure (by ref)"))
  (bind _bartendercharacter (message `/Game/Blueprint/Interfaces/BPI_PlayerCharacter.GetBartenderCharacter` OtherActor))
  (set `self.Character Ref` _bartendercharacter)
  (`self.SlowDown`))

(event `self.Box.OnComponentEndOverlap`
  (params (OverlappedComponent :type "PrimitiveComponent Object Reference") (OtherActor :type "Actor Object Reference") (OtherComp :type "PrimitiveComponent Object Reference") (OtherBodyIndex :type Integer))
  (bind _bartendercharacter (message `/Game/Blueprint/Interfaces/BPI_PlayerCharacter.GetBartenderCharacter` OtherActor))
  (set `CharacterMovementComponent.MaxWalkSpeed` 600.0 (`Character.CharacterMovement` _bartendercharacter)))

(event `SlowDown`
  (bind (_direction _speed) (`Timeline|WaterSlowDown`)
    (:`Update`
      (set `CharacterMovementComponent.MaxWalkSpeed` _speed (`Character.CharacterMovement` (`self.Character Ref`))))))

(event `Speed Up`
  (bind (_direction _speed) (`Timeline|WaterSpeedUp`)
    (:`Update`
      (set `CharacterMovementComponent.MaxWalkSpeed` _speed (`Character.CharacterMovement` (`self.Character Ref`))))))

(fn `UserConstructionScript`)