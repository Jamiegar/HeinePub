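; Blueprint function library that gives global access to the order system for servable orders.
; It exposes two functions, one to check whether an item is in the active orders and one to remove an item from them.
; Both fetch the pub game mode through an interface message on the current game mode, forward the call to its OrderManager and return the result.
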(fn `IsItemInActiveOrders`
  (params (ServableOrder :type "/Game/Blueprint/Items/ItemData/DA_ServeableItem Object Reference"))
  (returns (ItemIsInOrder :type Boolean))
  (bind _gamemode (message `/Game/Blueprint/Interfaces/BPI_PubGameMode.GetPubGameMode` (`GameplayStatics.GetGameMode` (`local.__WorldContext`))))
  (bind _itemisinorder (`/Game/Blueprint/GameMode/Managers/BP_OrderManager.IsItemInActiveOrders` (`/Game/Blueprint/GameMode/BP_HeinePub_GM.OrderManager` _gamemode) (`local.ServableOrder`)))
  (return _itemisinorder))

(fn `RemoveOrderFromActiveOrders`
  (params (RemoveItem :type "/Game/Blueprint/Items/ItemData/DA_ServeableItem Object Reference"))
  (returns (OrderWasRemoved :type Boolean))
  (bind _gamemode (message `/Game/Blueprint/Interfaces/BPI_PubGameMode.GetPubGameMode` (`GameplayStatics.GetGameMode` (`local.__WorldContext`))))
  (bind _hasremoveditem (`/Game/Blueprint/GameMode/Managers/BP_OrderManager.RemoveFromActiveOrders` (`/Game/Blueprint/GameMode/BP_HeinePub_GM.OrderManager` _gamemode) (`local.RemoveItem`)))
  (return _hasremoveditem))