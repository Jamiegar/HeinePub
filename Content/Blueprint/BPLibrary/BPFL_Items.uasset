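; Blueprint function library of item helpers for comparing items and checking whether an actor holds a required one.
; AreItemsEqual treats two valid items as equal when their ItemDisplayName matches, rather than comparing object references.
; RequireItemFromActor finds the actor's COM_ItemHolder component and returns true only if it holds an item that AreItemsEqual matches to the required one.
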(fn `AreItemsEqual`
  (params (`Item 1` :type "/Game/Blueprint/Items/ItemData/DA_ItemData Object Reference") (`Item 2` :type "/Game/Blueprint/Items/ItemData/DA_ItemData Object Reference"))
  (returns (isEqualItems :type Boolean))
  (if (and (`KismetSystemLibrary.IsValid` `Item 1`) (`KismetSystemLibrary.IsValid` `Item 2`))
    (return (`KismetStringLibrary.EqualEqual_StrStr` (`/Game/Blueprint/Items/ItemData/DA_ItemData.ItemDisplayName` `Item 1`) (`/Game/Blueprint/Items/ItemData/DA_ItemData.ItemDisplayName` `Item 2`)))))

(fn `RequireItemFromActor`
  (params (RequiredItem :type "/Game/Blueprint/Items/ItemData/DA_ItemData Object Reference") (Actor :type "Actor Object Reference"))
  (returns (ActorHasRequiredItem :type Boolean))
  (locals (ItemHolder :type "/Game/Blueprint/WorkStations/COM_ItemHolder Object Reference"))
  (bind _returnvalue (`Actor.GetComponentByClass` Actor "/Game/Blueprint/WorkStations/COM_ItemHolder.COM_ItemHolder_C"))
  (`/Engine/EditorBlueprintResources/StandardMacros.IsValid` _returnvalue
    (:`Is Valid`
      (bind _output_get (set `local.ItemHolder` _returnvalue))
      (if (`/Game/Blueprint/WorkStations/COM_ItemHolder.IsHoldingItem` _output_get)
        (if (`self.AreItemsEqual` (`/Game/Blueprint/WorkStations/COM_ItemHolder.GetHeldItem` (`local.ItemHolder`)) (`local.RequiredItem`) (`local.__WorldContext`))
          (return true)
          (else
            (return false)))
        (else
          (return false))))
    (:`Is Not Valid`
      (return false))))