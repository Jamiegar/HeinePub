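; Blueprint function library that gives quick access to specific UI widgets from anywhere in the game.
; Each getter fetches the UI manager through the game mode's GetUIManagerMessage call and reads its MasterUI.
; It exposes the bar fight and money widgets held by that master UI.
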(fn `GetBarFightUI`
  (returns (BarFightUI :type "/Game/Blueprint/UI/Game/GameplayUI/UI_BarFight Object Reference"))
  (bind _uimanager (message `/Game/Blueprint/Interfaces/BPI_PubGameMode.GetUIManager` (`GameplayStatics.GetGameMode` (`local.__WorldContext`))))
  (return (`/Game/Blueprint/UI/Game/GameplayUI/UI_GameplayMaster.UI_BarFight` (`/Game/Blueprint/GameMode/Managers/BP_UIManager.MasterUI` _uimanager))))

(fn `GetMoneyUI`
  (returns (MoneyUI :type "/Game/Blueprint/UI/Game/GameplayUI/UI_Money Object Reference"))
  (bind _uimanager (message `/Game/Blueprint/Interfaces/BPI_PubGameMode.GetUIManager` (`GameplayStatics.GetGameMode` (`local.__WorldContext`))))
  (return (`/Game/Blueprint/UI/Game/GameplayUI/UI_GameplayMaster.UI_Money` (`/Game/Blueprint/GameMode/Managers/BP_UIManager.MasterUI` _uimanager))))