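; Main menu game mode that runs the opening sequence as a small state machine: Initalize, Intro, then PresentMenu.
; It views through the level's BP_ViewportCamera, nudging it along X with a timeline during a fade-in.
; When the fade ends, it shows the start screen widget with mouse input and plays menu music.
; LoadLevel stops the music, clears widgets, fades out with audio and opens the named level.
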(event `self.ReceiveBeginPlay`
  (`self.ChangeGameState` "NewEnumerator0"))

(event `Initalize`
  (`self.SetUpViewportCamera`)
  (`self.ChangeGameState` "NewEnumerator1"))

(event `Intro`
  (`self.SetUpCameraLocation`)
  (`/Game/Blueprint/BPLibrary/BPFL_Camera.StartCameraFade` (delegate `OnFadeFinished`) 1.0 0.0 3.5 (struct) true true)
  (bind (_direction _alpha) (`Timeline|LerpToLocation` :!via `PlayFromStart`)
    (:`Update`
      (`self.K2_SetActorLocation` (`self.ViewportCamera`) (`KismetMathLibrary.VLerp` (`self.StartingLocation`) (`self.EndCameraLocation`) _alpha) false false))))

(event `OnFadeFinished`
  (`self.ChangeGameState` "NewEnumerator2"))

(event `PresentMenu`
  (bind _returnvalue (`GameplayStatics.GetPlayerController` 0))
  (bind _returnvalue_2 (`|CreateWidget` "/Game/Blueprint/UI/Menus/MainMenu/UI_StartScreen.UI_StartScreen_C"))
  (`UserWidget.AddToViewport` _returnvalue_2 0)
  (set `PlayerController.bShowMouseCursor` true _returnvalue)
  (`WidgetBlueprintLibrary.SetInputMode_GameAndUIEx` _returnvalue (`/Game/Blueprint/UI/Menus/MainMenu/UI_StartScreen.Button_0` _returnvalue_2))
  (bind _returnvalue_3 (`GameplayStatics.SpawnSound2D` "/Game/HeniePub_Music_Level_v1_Cue.HeniePub_Music_Level_v1_Cue" 1.0 1.0 0.0 null))
  (bind _output_get (set `self.MenuMusicRef` _returnvalue_3))
  (`AudioComponent.Play` _output_get 0.0))

(event `/Game/Blueprint/Interfaces/BPI_MenuGameMode.LoadLevel`
  (params (LevelName :type Name))
  (`AudioComponent.StopDelayed` (`self.MenuMusicRef`) 2.0)
  (`WidgetLayoutLibrary.RemoveAllWidgets`)
  (`/Game/Blueprint/BPLibrary/BPFL_Camera.StartCameraFade` (delegate `OnFadeFinished`) 0.0 1.0 1.5 (struct) true true))

(event `OnFadeFinished`
  (`GameplayStatics.OpenLevel` (stale `/Game/Blueprint/Interfaces/BPI_MenuGameMode.LoadLevel` LevelName))
  (`KismetSystemLibrary.PrintString` (`KismetStringLibrary.Conv_NameToString` (stale `/Game/Blueprint/Interfaces/BPI_MenuGameMode.LoadLevel` LevelName))))

(fn `ChangeGameState`
  (params (NewState :type "/Game/Blueprint/GameMode/MainMenu/E_MenuStates Enum" :default "NewEnumerator0"))
  (bind _output_get (set `self.CurrentState` NewState))
  (switch `/Game/Blueprint/GameMode/MainMenu/E_MenuStates` _output_get
    (:`NewEnumerator0`
      (`self.Initalize`))
    (:`NewEnumerator1`
      (`self.Intro`))
    (:`NewEnumerator2`
      (`self.PresentMenu`))))

(fn `SetUpCameraLocation`
  (bind _returnvalue (`self.K2_GetActorLocation` (`self.ViewportCamera`)))
  (set `self.StartingLocation` _returnvalue)
  (set `self.EndCameraLocation` (+ _returnvalue (75.0 0.0 0.0))))

(fn `SetUpViewportCamera`
  (bind _returnvalue (`GameplayStatics.GetActorOfClass` "/Game/Blueprint/Characters/Camera/BP_ViewportCamera.BP_ViewportCamera_C"))
  (bind _output_get (set `self.ViewportCamera` _returnvalue))
  (`PlayerController.SetViewTargetWithBlend` (`GameplayStatics.GetPlayerController` 0) _output_get 0.0 "VTBlend_Linear" 0.0 false))

(fn `UserConstructionScript`)