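; Order manager that releases scheduled item orders during a match and tracks which are active.
; Init copies the schedule from OrderData and binds to UI manager game time updates, adding the next row's items once elapsed game time reaches that row.
; Active orders are stored as an item-to-quantity map, with add and remove functions updating the order UI and a query for item membership.
; The construction script prints an error when OrderData is missing.
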(event `/Game/Blueprint/Interfaces/BPI_Initalizable.Init`
  (set `self.Game Orders` (`/Game/Blueprint/GameMode/OrderSystem/DA_GameOrders.GameOrders` (`self.OrderData`)))
  (set `self.ActiveRowIndex` 0)
  (bind _uimanager (message `/Game/Blueprint/Interfaces/BPI_PubGameMode.GetUIManager` (`GameplayStatics.GetGameMode`)))
  (add `/Game/Blueprint/GameMode/Managers/BP_UIManager.UpdateGameTime` _uimanager (`|CreateDelegate` :!event `OnGameTimeUpdated`)))

(fn `AddToActiveOrders`
  (params (OrderedItem :type "/Game/Blueprint/Items/ItemData/DA_ServeableItem Object Reference"))
  (locals (TempCurrentQuanity :type Integer))
  (if (`BlueprintMapLibrary.Map_Contains` (`self.ActiveOrders`) OrderedItem)
    (set `local.TempCurrentQuanity` (`BlueprintMapLibrary.Map_Find` (`self.ActiveOrders`) (`local.OrderedItem`)))
    (`BlueprintMapLibrary.Map_Remove` (`self.ActiveOrders`) (`local.OrderedItem`))
    (bind _result (`/Engine/EditorBlueprintResources/StandardMacros.IncrementInt` (`local.TempCurrentQuanity`))
      (:`  `
        (`BlueprintMapLibrary.Map_Add` (`self.ActiveOrders`) (`local.OrderedItem`) _result)))
    (else
      (`BlueprintMapLibrary.Map_Add` (`self.ActiveOrders`) (`local.OrderedItem`) 1)))
  (`/Game/Blueprint/UI/Game/GameplayUI/UI_Order.AddOrder` (`/Game/Blueprint/BPLibrary/BPFL_UserInterface.GetOrderUI`) (`local.OrderedItem`)))

(fn `IsItemInActiveOrders`
  (params (OrderItem :type "/Game/Blueprint/Items/ItemData/DA_ServeableItem Object Reference"))
  (returns (ItemIsInOrder :type Boolean))
  (return (`BlueprintMapLibrary.Map_Contains` (`self.ActiveOrders`) OrderItem)))

(fn `OnGameTimeUpdated`
  (params (RemainingMinutes :type "Float (double-precision)") (RemaingSeconds :type "Float (double-precision)") (GameRunningDuration :type "Float (double-precision)"))
  (bind (_gametime _items) (break `/Game/Blueprint/GameMode/OrderSystem/S_OrderData` (`|GetArrayItem` (`self.Game Orders`) (`self.ActiveRowIndex`))))
  (if (>= GameRunningDuration _gametime)
    (for _array_element _items
      (bind (_item _quanity) (break `/Game/Blueprint/GameMode/OrderSystem/S_ItemOrder` _array_element))
      (for _ (range 1 (+ _quanity 1))
        (`self.AddToActiveOrders` _item)))
    (`/Engine/EditorBlueprintResources/StandardMacros.IncrementInt` (`self.ActiveRowIndex`))))

(fn `RemoveFromActiveOrders`
  (params (RemovedItem :type "/Game/Blueprint/Items/ItemData/DA_ServeableItem Object Reference"))
  (returns (HasRemovedItem :type Boolean))
  (locals (TempItemQuantity :type Integer))
  (if (`BlueprintMapLibrary.Map_Contains` (`self.ActiveOrders`) RemovedItem)
    (set `local.TempItemQuantity` (`BlueprintMapLibrary.Map_Find` (`self.ActiveOrders`) (`local.RemovedItem`)))
    (`BlueprintMapLibrary.Map_Remove` (`self.ActiveOrders`) (`local.RemovedItem`))
    (bind _result (`/Engine/EditorBlueprintResources/StandardMacros.DecrementInt` (`local.TempItemQuantity`))
      (:`  `
        (if (<= _result 0)
          (`/Game/Blueprint/UI/Game/GameplayUI/UI_Order.Remove Order With Item` (`/Game/Blueprint/BPLibrary/BPFL_UserInterface.GetOrderUI`) (`local.RemovedItem`))
          (return true)
          (else
            (`BlueprintMapLibrary.Map_Add` (`self.ActiveOrders`) (`local.RemovedItem`) (`local.TempItemQuantity`))
            (`/Game/Blueprint/UI/Game/GameplayUI/UI_Order.Remove Order With Item` (`/Game/Blueprint/BPLibrary/BPFL_UserInterface.GetOrderUI`) (`local.RemovedItem`))
            (return true)))))
    (else
      (return false))))

(fn `UserConstructionScript`
  (`parent.UserConstructionScript`)
  (`/Engine/EditorBlueprintResources/StandardMacros.IsValid` (`self.OrderData`)
    (:`Is Not Valid`
      (`KismetSystemLibrary.PrintString` "ERROR: Add data order " true true (struct :`R` 1.0 :`G` 0.010323 :`A` 1.0)))))