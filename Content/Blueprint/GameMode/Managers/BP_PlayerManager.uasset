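; Player manager that sets up local multiplayer, creating a controller and a bartender character for each player.
; Init recreates local players, spawns characters at PlayerStart transforms, then possesses them with input disabled and every view set to one shared viewport camera.
; It binds to the game state's change event and re-enables character input on Start Game.
; Separate functions gather the PlayerStarts and viewport camera, but Init does not call them.
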(event `/Game/Blueprint/Interfaces/BPI_Initalizable.Init`
  (`self.SetUpPlayerController`)
  (`self.SetUpPlayerCharacter`)
  (`self.ControllerPossessPlayer`)
  (`/Game/Blueprint/Characters/PlayerPawns/BP_PlayerCharacterBarTender.SetMappingContext` (`self.PlayerCharacter`))
  (bind _gamestate (message `/Game/Blueprint/Interfaces/BPI_GameStates.GetGameState` (`GameplayStatics.GetGameState`)))
  (add `/Game/Blueprint/GameMode/BP_HeinePub_GS.OnGameStateChanged` _gamestate (`|CreateDelegate` :!event `OnGameStateChanged`)))

(event `OnGameStateChanged`
  (params (NewGameState :type "/Game/Blueprint/GameMode/Enum_GameStates Enum" :default "NewEnumerator4"))
  (switch `/Game/Blueprint/GameMode/Enum_GameStates` NewGameState
    (:`NewEnumerator2`
      (`self.EnableCharcterInput`))))

(fn `ControllerPossessPlayer`
  (locals (Controller :type "/Game/Blueprint/Characters/PlayerController/BP_PlayerPubController Object Reference"))
  (for (_array_element _array_index) (`self.PlayerController`)
    (bind _output_get (set `local.Controller` _array_element))
    (bind _output (`|GetArrayItem` (`self.PlayerCharacter`) _array_index))
    (`Controller.Possess` _output_get _output)
    (`self.DisableInput` _output (`local.Controller`))
    (`PlayerController.SetViewTargetWithBlend` (`local.Controller`) (`self.ViewportCamera`) 0.0 "VTBlend_Linear" 0.0 false)))

(fn `EnableCharcterInput`
  (for (_array_element _array_index) (`self.PlayerCharacter`)
    (`self.EnableInput` _array_element (`|GetArrayItem` (`self.PlayerController`) _array_index))))

(fn `GetPlayerStarts`
  (bind _outactors (`GameplayStatics.GetAllActorsOfClass` "/Script/Engine.PlayerStart"))
  (set `self.PlayerStarts` _outactors))

(fn `GetViewportCamera`
  (bind _returnvalue (`GameplayStatics.GetActorOfClass` "/Game/Blueprint/Characters/Camera/BP_ViewportCamera.BP_ViewportCamera_C"))
  (`/Engine/EditorBlueprintResources/StandardMacros.IsValid` _returnvalue
    (:`Is Valid`
      (set `self.ViewportCamera` _returnvalue))
    (:`Is Not Valid`
      (`KismetSystemLibrary.PrintString` "Error: No Viewport Camera" true true (struct :`R` 1.0 :`G` 0.015568 :`A` 1.0)))))

(fn `SetUpPlayerCharacter`
  (for (_ _array_index) (`self.PlayerController`)
    (bind _returnvalue (`|SpawnActorFromClass` "/Game/Blueprint/Characters/PlayerPawns/BP_PlayerCharacterBarTender.BP_PlayerCharacterBarTender_C" (`self.GetTransform` (`|GetArrayItem` (`self.PlayerStarts`) _array_index)) "Undefined" "OverrideRootScale" null null))
    (`KismetArrayLibrary.Array_Add` (`self.PlayerCharacter`) _returnvalue)
    (message `/Game/Blueprint/Interfaces/BPI_Initalizable.Init` _returnvalue)))

(fn `SetUpPlayerController`
  (`GameplayStatics.RemovePlayer` (`GameplayStatics.GetPlayerController` 0))
  (for _index (range (`self.NumberOfPlayers`))
    (bind _returnvalue (`GameplayStatics.CreatePlayer` _index))
    (message `/Game/Blueprint/Interfaces/BPI_Initalizable.Init` _returnvalue)
    (bind _controller (message `/Game/Blueprint/Interfaces/BPI_PubPlayerController.GetPubPlayerController` _returnvalue))
    (`KismetArrayLibrary.Array_Add` (`self.PlayerController`) _controller)))

(fn `UserConstructionScript`
  (`parent.UserConstructionScript`))