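; BP_UIManager is a manager Blueprint that builds the game's HUD and runs the match countdown clock.
; Init creates the game time, money, order time and bar fight widgets and adds each to the viewport.
; A looping one-second timer decrements minutes and seconds, pushes them to the time widget, and clears itself when time runs out.
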(event `/Game/Blueprint/Interfaces/BPI_Initalizable.Init`
  ;[1 1 1] Init
  (`self.CreateGameTimeUI`)
  (`self.CreateMoneyUI`)
  (`self.CreateOrderTimeUI`)
  (`self.CreateBarFightUI`))

(event `CreateGameTimeUI`
  ;[1 1 1] GameTimeUI
  (`self.SetUpGameTimeUI`)
  (bind _returnvalue (`KismetSystemLibrary.K2_SetTimerDelegate` (delegate `GameTimer`) 1.0 true))
  (set `self.GameTimerHandle` _returnvalue))

(event `GameTimer`
  ;[1 1 1] GameTimeUI
  (`self.RunGameTimer`))

(event `CreateMoneyUI`
  ;[1 1 1] MoneyUI
  (`self.SetUpMoneyUI`))

(event `CreateOrderTimeUI`
  ;[1 1 1] OrderTimeUI
  (`self.SetUpOrderTimeUI`))

(event `CreateBarFightUI`
  ;[1 1 1] BarFightUI
  (`self.SetUpBarFightUI`))

(fn `RunGameTimer`
  (bind _result (`/Engine/EditorBlueprintResources/StandardMacros.DecrementFloat` (`self.TimeSeconds`))
    (:`  `
      (`self.SecondsBelow0?` _result
        (:`True`
          (`/Engine/EditorBlueprintResources/StandardMacros.DecrementFloat` (`self.TimeMinutes`)
            (:`  `
              _)))
        (:`False`
          _))
      (`/Game/Blueprint/UI/Game/UI_GameTime.UpdateTime` (`self.UI_GameTimer`) (`self.TimeMinutes`) (`self.TimeSeconds`))
      (`self.TimeUp?`
        (:`true`
          (`KismetSystemLibrary.K2_ClearAndInvalidateTimerHandle` (`self.GameTimerHandle`)))))))

(fn `SetUpBarFightUI`
  (bind _returnvalue (`|GenericCreateObject` "/Game/Blueprint/UI/Game/UI_BarFight.UI_BarFight_C"))
  (bind _output_get (set `self.UI_BarFight` _returnvalue))
  (`UserWidget.AddToViewport` _output_get 0))

(fn `SetUpGameTimeUI`
  (bind _returnvalue (`|GenericCreateObject` "/Game/Blueprint/UI/Game/UI_GameTime.UI_GameTime_C"))
  (bind _output_get (set `self.UI_GameTimer` _returnvalue))
  (`UserWidget.AddToViewport` _output_get 0)
  (`/Game/Blueprint/UI/Game/UI_GameTime.UpdateTime` (`self.UI_GameTimer`) (`self.TimeMinutes`) (`self.TimeSeconds`)))

(fn `SetUpMoneyUI`
  (bind _returnvalue (`|GenericCreateObject` "/Game/Blueprint/UI/Game/UI_Money.UI_Money_C"))
  (bind _output_get (set `self.UI_Money` _returnvalue))
  (`UserWidget.AddToViewport` _output_get 0))

(fn `SetUpOrderTimeUI`
  (bind _returnvalue (`|GenericCreateObject` "/Game/Blueprint/UI/Game/UI_OrderTime.UI_OrderTime_C"))
  (bind _output_get (set `self.UI_OrderTime` _returnvalue))
  (`UserWidget.AddToViewport` _output_get 0)
  (`/Game/Blueprint/UI/Game/UI_OrderTime.Init` (`self.UI_OrderTime`)))

(fn `UserConstructionScript`
  (`parent.UserConstructionScript`))