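; BP_FightManager is a game-mode manager for bar fights, tracking whether one is ongoing and what it costs.
; When the game state changes to Start Game, it binds to the bar fight UI's started event.
; Each fight activates a reused fight-dust Niagara effect and compounds the cost by an incrementing multiplier.
; StopBarFight resets the UI meter and deactivates the effect; the timer function is an unfinished stub.
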(event `/Game/Blueprint/Interfaces/BPI_Initalizable.Init`
  (bind _gamestate (message `/Game/Blueprint/Interfaces/BPI_GameStates.GetGameState` (`GameplayStatics.GetGameState`)))
  (add `/Game/Blueprint/GameMode/BP_HeinePub_GS.OnGameStateChanged` _gamestate (`|CreateDelegate` :!event `OnGameStateChanaged`)))

(event `OnGameStateChanaged`
  (params (NewGameState :type "/Game/Blueprint/GameMode/Enum_GameStates Enum" :default "NewEnumerator4"))
  (switch `/Game/Blueprint/GameMode/Enum_GameStates` NewGameState
    (:`NewEnumerator2`
      (bind _output_get (set `self.Bar Fight UI` (`/Game/Blueprint/BPLibrary/BPFL_UserInterface.GetBarFightUI`)))
      (add `/Game/Blueprint/UI/Game/GameplayUI/UI_BarFight.OnBarFightStarted` _output_get (`|CreateDelegate` :!event `OnBarFightStarted`)))))

(event `OnBarFightStarted`
  (set `self.OnGoingBarFight` true)
  (`self.SpawnBarFightVFX`)
  (`self.CalcBarFightCost`))

(event `StopBarFight`
  (if (`self.OnGoingBarFight`)
    (set `self.OnGoingBarFight` false)
    (`/Game/Blueprint/UI/Game/GameplayUI/UI_BarFight.RestBarFightMeter` (`self.Bar Fight UI`))
    (`ActorComponent.Deactivate` (`self.BarFightVFX`))))

(fn `BeginBarFightTimer`)

(fn `CalcBarFightCost`
  (bind _result (`/Engine/EditorBlueprintResources/StandardMacros.IncrementFloat` (`self.BarFightMultiplier`))
    (:`  `
      (set `self.BarFightCost` (* _result (`self.BarFightCost`))))))

(fn `GetBarFightCost`
  (returns (Cost :type "Float (double-precision)"))
  (return (`self.BarFightCost`)))

(fn `SpawnBarFightVFX`
  (`/Engine/EditorBlueprintResources/StandardMacros.IsValid` (`self.BarFightVFX`)
    (:`Is Valid`
      (`ActorComponent.Activate` (`self.BarFightVFX`) true))
    (:`Is Not Valid`
      (bind _returnvalue (`NiagaraFunctionLibrary.SpawnSystemAtLocation` "/Game/Blueprint/Niagra/Emiters/NE_FightDust_System.NE_FightDust_System" (`KismetMathLibrary.TransformLocation` (`self.GetTransform`) (`self.FightStartingPosition`))))
      (set `self.BarFightVFX` _returnvalue))))

(fn `UserConstructionScript`
  (`parent.UserConstructionScript`))