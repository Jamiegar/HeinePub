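; BP_TimerManager runs the match countdown clock and shows it on screen.
; Init creates the UI_GameTime widget, adds it to the viewport and starts a looping one-second timer.
; Each tick decrements seconds, rolls into minutes through the SecondsBelow0 macro, refreshes the widget and clears the timer when TimeUp reports zero.
; Reaching zero only stops the clock; no end-of-game event is fired here.
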(event `/Game/Blueprint/Interfaces/BPI_Initalizable.Init`
  (`self.SetUpTimeUI`)
  (bind _returnvalue (`KismetSystemLibrary.K2_SetTimerDelegate` (delegate `GameTimer`) 1.0 true))
  (set `self.GameTimerHandle` _returnvalue))

(event `GameTimer`
  (`self.RunGameTimer`))

(fn `RunGameTimer`
  (bind _result (`/Engine/EditorBlueprintResources/StandardMacros.DecrementFloat` (`self.TimeSeconds`))
    (:`  `
      (`self.SecondsBelow0?` _result
        (:`True`
          (`/Engine/EditorBlueprintResources/StandardMacros.DecrementFloat` (`self.TimeMinutes`)
            (:`  `
              _)))
        (:`False`
          _))
      (`/Game/Blueprint/UI/Game/GameplayUI/UI_GameTime.UpdateTime` (`self.UI_GameTimer`) (`self.TimeMinutes`) (`self.TimeSeconds`))
      (`self.TimeUp?`
        (:`true`
          (`KismetSystemLibrary.K2_ClearAndInvalidateTimerHandle` (`self.GameTimerHandle`)))))))

(fn `SetUpTimeUI`
  (bind _returnvalue (`|GenericCreateObject` "/Game/Blueprint/UI/Game/GameplayUI/UI_GameTime.UI_GameTime_C"))
  (bind _output_get (set `self.UI_GameTimer` _returnvalue))
  (`UserWidget.AddToViewport` _output_get 0)
  (`/Game/Blueprint/UI/Game/GameplayUI/UI_GameTime.UpdateTime` (`self.UI_GameTimer`) (`self.TimeMinutes`) (`self.TimeSeconds`)))

(fn `UserConstructionScript`
  (`parent.UserConstructionScript`))