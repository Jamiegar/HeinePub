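; Tutorial game mode for a pub game, teaching glass, tap pouring, serving, binning and bar-fight bell mechanics.
; StartGame runs the parent start and sets a timer; TutorialInit pauses the game timer, which TutorialEnd resumes.
; Each stage mixes delayed popups with a level sequence that hides the master UI until finished, then schedules a timer event.
; Helper functions toggle movement for all player characters but are not called here.
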(event `self.StartGame`
  (`parent.StartGame`)
  (`KismetSystemLibrary.K2_SetTimerDelegate` (`|CreateDelegate` :!event `Tutorial Init`) 1.0))

(event `Tutorial Init`
  ;[1 0.005986 0.8643] Tutorial UI Pop up (Begining)
  (`KismetSystemLibrary.K2_PauseTimerHandle` (`/Game/Blueprint/GameMode/Managers/BP_UIManager.GameTimerHandle` (`self.UIManger`)))
  (`/Game/Blueprint/BPLibrary/BPFL_Tutorial.CreateTutorialPopup` "Welcome to the pub!" 4.0)
  (`KismetSystemLibrary.Delay` 4.5)
  (`/Game/Blueprint/BPLibrary/BPFL_Tutorial.CreateTutorialPopup` "Its your job to keep the drinks flowing and pub running" 5.0)
  (`KismetSystemLibrary.Delay` 5.5)
  (`/Game/Blueprint/BPLibrary/BPFL_Tutorial.CreateTutorialPopup` "To begin, you'll need to grab a glass, these can be found at the 'Glass' station" 5.0)
  (`KismetSystemLibrary.K2_SetTimerDelegate` (`|CreateDelegate` :!event `Tutoria Glassl Level Sequence`) 5.5))

(event `Tutoria Glassl Level Sequence`
  ;[1 1 1] Glass Station Tutorial
  (bind (_outactor _returnvalue) (`LevelSequencePlayer.CreateLevelSequencePlayer` (`|GetArrayItem` (`self.Level Sequence Film`)) (`self.Level Sequence Settings`)))
  (`MovieSceneSequencePlayer.Play` _returnvalue)
  (add `MovieSceneSequencePlayer.OnFinished` _returnvalue (delegate `Finished Glass`))
  (`Widget.SetVisibility` (`/Game/Blueprint/GameMode/Managers/BP_UIManager.MasterUI` (`self.UIManger`)) "Hidden"))

(event `Finished Glass`
  ;[1 1 1] Glass Station Tutorial
  (`Widget.SetVisibility` (`/Game/Blueprint/GameMode/Managers/BP_UIManager.MasterUI` (`self.UIManger`)) "Visible")
  (`KismetSystemLibrary.Delay` 0.5)
  (`/Game/Blueprint/BPLibrary/BPFL_Tutorial.CreateTutorialPopup` "Grab a glass by pressing 'A' or left mouse button next to the Station" 5.0)
  (`KismetSystemLibrary.Delay` 10.5)
  (`/Game/Blueprint/BPLibrary/BPFL_Tutorial.CreateTutorialPopup` "Next you'll need to fill it with the finest beverage" 5.0)
  (`KismetSystemLibrary.K2_SetTimerDelegate` (`|CreateDelegate` :!event `Tutorial Tap Level Sequence`) 6.0))

(event `Tutorial Tap Level Sequence`
  ;[1 1 1] Tap Tutorial
  (bind (_outactor _returnvalue) (`LevelSequencePlayer.CreateLevelSequencePlayer` (`|GetArrayItem` (`self.Level Sequence Film`) 1) (`self.Level Sequence Settings`)))
  (`MovieSceneSequencePlayer.Play` _returnvalue)
  (add `MovieSceneSequencePlayer.OnFinished` _returnvalue (delegate `Finished Tap`))
  (`Widget.SetVisibility` (`/Game/Blueprint/GameMode/Managers/BP_UIManager.MasterUI` (`self.UIManger`)) "Hidden"))

(event `Finished Tap`
  ;[1 1 1] Tap Tutorial
  (`Widget.SetVisibility` (`/Game/Blueprint/GameMode/Managers/BP_UIManager.MasterUI` (`self.UIManger`)) "Visible")
  (`KismetSystemLibrary.Delay` 0.5)
  (`/Game/Blueprint/BPLibrary/BPFL_Tutorial.CreateTutorialPopup` "Head on over to the 'Tap' and fill your glass" 6.0)
  (`KismetSystemLibrary.Delay` 6.5)
  (`/Game/Blueprint/BPLibrary/BPFL_Tutorial.CreateTutorialPopup` "Pouring is more than a mere skill, it's an art!" 4.0)
  (`KismetSystemLibrary.Delay` 4.5)
  (`/Game/Blueprint/BPLibrary/BPFL_Tutorial.CreateTutorialPopup` "First pick the beverage the customer wants, then interact again to pour" 5.0)
  (`KismetSystemLibrary.Delay` 10.0)
  (`/Game/Blueprint/BPLibrary/BPFL_Tutorial.CreateTutorialPopup` "Landing in the red will result in a bad pint and upset the customer. Landing in the Green will result in a Good pint leaving no negative effects. Landing in the purple will result in a 'Perfect Pint' calming the customer and earning more money!" 8.0)
  (`KismetSystemLibrary.K2_SetTimerDelegate` (`|CreateDelegate` :!event `Tutorial Level Sequence Serve`) 8.0))

(event `Tutorial Level Sequence Serve`
  ;[1 1 1] Serve Tutorial
  (bind (_outactor _returnvalue) (`LevelSequencePlayer.CreateLevelSequencePlayer` (`|GetArrayItem` (`self.Level Sequence Film`) 2) (`self.Level Sequence Settings`)))
  (`MovieSceneSequencePlayer.Play` _returnvalue)
  (add `MovieSceneSequencePlayer.OnFinished` _returnvalue (delegate `FinishedServe`))
  (`Widget.SetVisibility` (`/Game/Blueprint/GameMode/Managers/BP_UIManager.MasterUI` (`self.UIManger`)) "Hidden"))

(event `FinishedServe`
  ;[1 1 1] Serve Tutorial
  (`Widget.SetVisibility` (`/Game/Blueprint/GameMode/Managers/BP_UIManager.MasterUI` (`self.UIManger`)) "Visible")
  (`KismetSystemLibrary.Delay` 0.5)
  (`/Game/Blueprint/BPLibrary/BPFL_Tutorial.CreateTutorialPopup` "Once poured, head over to the serving area to hand over your beer" 5.0)
  (`KismetSystemLibrary.Delay` 5.5)
  (`/Game/Blueprint/BPLibrary/BPFL_Tutorial.CreateTutorialPopup` "Once handed over, you'll recieve money depending on timing and your pouring skill" 5.0)
  (`KismetSystemLibrary.Delay` 5.5)
  (`/Game/Blueprint/BPLibrary/BPFL_Tutorial.CreateTutorialPopup` "Complete orders when they come in at the top to stay ahead. Be careful though, as difficulty will ramp with time" 5.0)
  (`KismetSystemLibrary.Delay` 5.5)
  (`/Game/Blueprint/BPLibrary/BPFL_Tutorial.CreateTutorialPopup` "If you don't like the pint you've poured, you can always bin it and start again" 5.0)
  (`KismetSystemLibrary.K2_SetTimerDelegate` (`|CreateDelegate` :!event `Totorial Bin Sequence`) 5.5))

(event `Totorial Bin Sequence`
  ;[1 1 1] Bin Tutorial
  (bind (_outactor _returnvalue) (`LevelSequencePlayer.CreateLevelSequencePlayer` (`|GetArrayItem` (`self.Level Sequence Film`) 3) (`self.Level Sequence Settings`)))
  (`MovieSceneSequencePlayer.Play` _returnvalue)
  (add `MovieSceneSequencePlayer.OnFinished` _returnvalue (delegate `FinishedBin`))
  (`Widget.SetVisibility` (`/Game/Blueprint/GameMode/Managers/BP_UIManager.MasterUI` (`self.UIManger`)) "Hidden"))

(event `FinishedBin`
  ;[1 1 1] Bin Tutorial
  (`Widget.SetVisibility` (`/Game/Blueprint/GameMode/Managers/BP_UIManager.MasterUI` (`self.UIManger`)) "Visible")
  (`KismetSystemLibrary.Delay` 0.5)
  (`/Game/Blueprint/BPLibrary/BPFL_Tutorial.CreateTutorialPopup` "Binning your pint will clear the glass but will require time to do so" 5.0)
  (`KismetSystemLibrary.K2_SetTimerDelegate` (`|CreateDelegate` :!event `Tutorial Bar Fight Sequence`) 5.5))

(event `Tutorial Bar Fight Sequence`
  ;[1 1 1] Bar Fight Tutorial
  (`/Game/Blueprint/BPLibrary/BPFL_Tutorial.CreateTutorialPopup` "Failing to make complete an order in time or serving a bad pint will increase the chance of a bar fight happening!" 5.0)
  (`KismetSystemLibrary.Delay` 5.5)
  (`/Game/Blueprint/BPLibrary/BPFL_Tutorial.CreateTutorialPopup` "Bar fights will cause you to go bust unless resolved." 4.0)
  (`KismetSystemLibrary.Delay` 4.5)
  (`/Game/Blueprint/BPLibrary/BPFL_Tutorial.CreateTutorialPopup` "Clearing the bar fight can be done by ringing the 'bell', which will cost money at an increasing rate" 5.0)
  (`KismetSystemLibrary.Delay` 5.5)
  (bind (_outactor _returnvalue) (`LevelSequencePlayer.CreateLevelSequencePlayer` (`|GetArrayItem` (`self.Level Sequence Film`) 4) (`self.Level Sequence Settings`)))
  (`MovieSceneSequencePlayer.Play` _returnvalue)
  (add `MovieSceneSequencePlayer.OnFinished` _returnvalue (delegate `FinishedBell`))
  (`Widget.SetVisibility` (`/Game/Blueprint/GameMode/Managers/BP_UIManager.MasterUI` (`self.UIManger`)) "Hidden"))

(event `FinishedBell`
  ;[1 1 1] Bar Fight Tutorial
  (`Widget.SetVisibility` (`/Game/Blueprint/GameMode/Managers/BP_UIManager.MasterUI` (`self.UIManger`)) "Visible")
  (`KismetSystemLibrary.K2_SetTimerDelegate` (`|CreateDelegate` :!event `Tutorial End`) 2.0))

(event `Tutorial End`
  ;[1 1 1] Game Start
  (`/Game/Blueprint/BPLibrary/BPFL_Tutorial.CreateTutorialPopup` "Enjoy and rack up as much monay as you can in time!" 5.0)
  (`KismetSystemLibrary.K2_UnPauseTimerHandle` (`/Game/Blueprint/GameMode/Managers/BP_UIManager.GameTimerHandle` (`self.UIManger`))))

(fn `Disable Player Movement`
  (for _array_element (`/Game/Blueprint/GameMode/Managers/BP_PlayerManager.PlayerCharacter` (`self.PlayerManager`))
    (`CharacterMovementComponent.DisableMovement` (`Character.CharacterMovement` _array_element))))

(fn `Enable Player Movement`
  (for _array_element (`/Game/Blueprint/GameMode/Managers/BP_PlayerManager.PlayerCharacter` (`self.PlayerManager`))
    (`CharacterMovementComponent.SetMovementMode` (`Character.CharacterMovement` _array_element) "MOVE_Walking" 0)))

(fn `UserConstructionScript`)