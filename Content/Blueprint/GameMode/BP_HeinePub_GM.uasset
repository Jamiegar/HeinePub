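; Game mode for the HeinePub level that bootstraps the game's managers and reacts to game state changes.
; It binds to game state change messages, and on Initialization finds the placed UI, player, order, fight and workstation managers, initializes and stores them, then requests pre-game.
; Missing managers print an error, while the pre-game and start handlers only print.
; Level loading clears widgets and fades out camera and audio before opening the named level.
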(event `self.ReceiveBeginPlay`
  (bind _gamestate (message `/Game/Blueprint/Interfaces/BPI_GameStates.GetGameState` (`GameplayStatics.GetGameState`)))
  (add `/Game/Blueprint/GameMode/BP_HeinePub_GS.OnGameStateChanged` _gamestate (`|CreateDelegate` :!event `OnGameStateChanged`))
  (message `/Game/Blueprint/Interfaces/BPI_Initalizable.Init` (`GameplayStatics.GetGameState`)) ; inits game state and starts \nInitialization
)

(event `Initialization`
  (`self.SetUpManager` "/Game/Blueprint/GameMode/Managers/BP_UIManager.BP_UIManager_C" (`self.UIManger`))
  (`self.SetUpManager` "/Game/Blueprint/GameMode/Managers/BP_PlayerManager.BP_PlayerManager_C" (`self.PlayerManager`))
  (`self.SetUpManager` "/Game/Blueprint/GameMode/Managers/BP_OrderManager.BP_OrderManager_C" (`self.OrderManager`))
  (`self.SetUpManager` "/Game/Blueprint/GameMode/Managers/BP_FightManager.BP_FightManager_C" (`self.FightManager`))
  (`self.SetUpManager` "/Game/Blueprint/GameMode/Managers/BP_WorkstationsManager.BP_WorkstationsManager_C" (`self.WorkstationsManager`))
  (message `/Game/Blueprint/Interfaces/BPI_GameStates.ChangeGameState` (`GameplayStatics.GetGameState`) "NewEnumerator1"))

(event `PreGame`
  (`KismetSystemLibrary.PrintString` "Pre-Game"))

(event `StartGame`
  (`KismetSystemLibrary.PrintString` "Start Game"))

(event `/Game/Blueprint/Interfaces/BPI_MenuGameMode.LoadLevel`
  (params (LevelName :type Name))
  (`WidgetLayoutLibrary.RemoveAllWidgets`)
  (`/Game/Blueprint/BPLibrary/BPFL_Camera.StartCameraFade` (delegate `OnFadeFinished`) 0.0 1.0 1.5 (struct) true true))

(event `OnFadeFinished`
  (`GameplayStatics.OpenLevel` (stale `/Game/Blueprint/Interfaces/BPI_MenuGameMode.LoadLevel` LevelName)))

(fn `GetPubGameMode`
  (returns (GameMode :type "/Game/Blueprint/GameMode/BP_HeinePub_GM Object Reference"))
  (return self))

(fn `GetUIManager`
  (returns (UIManager :type "/Game/Blueprint/GameMode/Managers/BP_UIManager Object Reference"))
  (return (`self.UIManger`)))

(fn `OnGameStateChanged`
  (params (NewGameState :type "/Game/Blueprint/GameMode/Enum_GameStates Enum" :default "NewEnumerator4"))
  (switch `/Game/Blueprint/GameMode/Enum_GameStates` NewGameState
    (:`NewEnumerator0`
      (`self.Initialization`))
    (:`NewEnumerator1`
      (`self.PreGame`))
    (:`NewEnumerator2`
      (`self.StartGame`))))

(fn `SetUpManager`
  (params (ManagerClassType :type "/Game/Blueprint/GameMode/Managers/BP_Manager Class Reference") (OutManagerVariable :type "/Game/Blueprint/GameMode/Managers/BP_Manager Object Reference (by ref)"))
  (locals (TempMangerResult :type "/Game/Blueprint/GameMode/Managers/BP_Manager Object Reference"))
  (bind _returnvalue (`GameplayStatics.GetActorOfClass` ManagerClassType))
  (bind _output_get (set `local.TempMangerResult` _returnvalue))
  (`/Engine/EditorBlueprintResources/StandardMacros.IsValid` _output_get
    (:`Is Valid`
      (message `/Game/Blueprint/Interfaces/BPI_Initalizable.Init` (`local.TempMangerResult`))
      (`|VariableSetRef` (`local.OutManagerVariable`) (`local.TempMangerResult`)))
    (:`Is Not Valid`
      (`KismetSystemLibrary.PrintString` (`KismetStringLibrary.Concat_StrStr` "Error: Manager of type (" (`KismetSystemLibrary.GetClassDisplayName` (`local.ManagerClassType`)) ") is not in level") true true (struct :`R` 1.0 :`A` 1.0)))))

(fn `UserConstructionScript`)